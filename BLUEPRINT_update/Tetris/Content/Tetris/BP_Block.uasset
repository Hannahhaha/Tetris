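; BP_Block is a four-mesh Tetris piece actor that handles its own rotation and collision checks.
; BlockRotation steps pitch in 90-degree increments up to RotMax, reverting through a RotRestore lookup when the new pose collides.
; DetectCollison box-traces each mesh on the Visibility channel, either in place for rotation or one 100-unit cell down, left or right.
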(event `self.ReceiveBeginPlay`
  (set `self.AllBlock` (`|MakeArray` (`self.Sm_Center`) (`self.Sm_01`) (`self.Sm_02`) (`self.Sm_03`))))

(event `BlockRotation`
  (bind _rot (`self.Rot`))
  ;[0.2552 0.2552 0.2552] 方块旋转
  (if (> (`self.RotMax`) 0)
    (set `self.Rot` (+ _rot 1))
    (if (> _rot (`self.RotMax`))
      (set `self.Rot` 0))
    (`self.K2_SetActorRotation` (`KismetMathLibrary.MakeRotator` 0.0 (`KismetMathLibrary.Conv_IntToDouble` (* (`self.Rot`) 90))))
    (bind _collision_ (`self.DetectCollison` true))
    (if _collision_
      (`self.K2_SetActorRotation` (`KismetMathLibrary.MakeRotator` 0.0 (`KismetMathLibrary.Conv_IntToDouble` (`|GetArrayItem` (`self.RotRestore`) (`self.Rot`)))))
      (set `self.Rot` (- (`self.Rot`) 1)))))

(fn `DetectCollison`
  (params (Rot :type Boolean) (Down :type Boolean) (Left :type Boolean))
  (returns (`Collision?` :type Boolean))
  (locals (L_Location :type "Vector Structure"))
  ;[0.2083 0.2083 0.2083] 碰撞检测
  (if Rot
    (set `local.L_Location` (0.0 0.0 0.0))
    (elif Down
      (set `local.L_Location` (0.0 0.0 100.0))
      (elif Left
        (set `local.L_Location` (100.0 0.0 0.0))
        (else
          (set `local.L_Location` (-100.0 0.0 0.0))))))
  (for _array_element (`self.AllBlock`)
    (bind _returnvalue (- (`SceneComponent.K2_GetComponentLocation` _array_element) (`local.L_Location`)))
    (bind (_outhit _returnvalue_2) (`KismetSystemLibrary.BoxTraceSingle` _returnvalue (+ _returnvalue (0.0 40.0 0.0)) (45.0 20.0 45.0) (struct) "TraceTypeQuery1"))
    (if _returnvalue_2
      (break)))
  (return _returnvalue_2))

(fn `UserConstructionScript`)